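; BP_Gate is a wormhole gate effect Blueprint that publishes the wormhole's position to materials.
; On BeginPlay it writes the world location of its LocatorWormhole component into the Position vector of the PC_Wormhole parameter collection, once, with no later updates.
; The construction script is empty, and its disconnected nodes for setting Position and Radius and printing the location never run.
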(event `self.ReceiveBeginPlay`
  (`KismetMaterialLibrary.SetVectorParameterValue` "/Game/Effects/Wormhole/PC_Wormhole.PC_Wormhole" "Position" (`KismetMathLibrary.Conv_VectorToLinearColor` (`SceneComponent.K2_GetComponentLocation` (`self.LocatorWormhole`)))))

(fn `UserConstructionScript`)